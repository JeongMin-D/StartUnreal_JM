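; BP_MoveLeftRight slides a Sphere component back and forth along its relative X axis, with movement toggled on and off by an event from a Pawn.
; Tick calls MoveRight or MoveLeft based on a direction flag, which each function flips at its fixed bound, scaling Speed by delta time.
; BeginPlay binds to the Pawn's ClickY dispatcher, apparently to the auto-generated function that toggles IsPlayMove.
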(event `self.ReceiveTick`
  (params (DeltaSeconds :type "Float (single-precision)"))
  (if (`self.IsPlayMove`)
    (if (`self.IsRightMove`)
      (`self.MoveRight` DeltaSeconds)
      (else
        (`self.MoveLeft` DeltaSeconds)))))

(event `self.ReceiveBeginPlay`
  (add `/Game/StartUnreal/BP_Pawn.EventDispatcher_ClickY` (`self.Pawn`) (`|CreateDelegate` :!event `BP_MoveLeftRight_AutoGenFunc`)))

(fn `BP_MoveLeftRight_AutoGenFunc`
  (set `self.IsPlayMove` (not (`self.IsPlayMove`))))

(fn `MoveLeft`
  (params (DeltaSeconds :type "Float (double-precision)"))
  (bind _sphere (`self.Sphere`))
  (bind _relativelocation_x (`KismetMathLibrary.BreakVector` (`SceneComponent.RelativeLocation` _sphere)))
  (bind _result (`/Engine/EditorBlueprintResources/StandardMacros.NegateFloat` (* DeltaSeconds (`self.Speed`)))
    (:`  `
      (`SceneComponent.K2_AddRelativeLocation` _sphere (`KismetMathLibrary.MakeVector` _result) false false)
      (if (<= _relativelocation_x 0.0)
        (set `self.IsRightMove` true)))))

(fn `MoveRight`
  (params (DeltaSeconds :type "Float (double-precision)"))
  (bind _sphere (`self.Sphere`))
  (bind _relativelocation_x (`KismetMathLibrary.BreakVector` (`SceneComponent.RelativeLocation` _sphere)))
  (`SceneComponent.K2_AddRelativeLocation` _sphere (`KismetMathLibrary.MakeVector` (* DeltaSeconds (`self.Speed`))) false false)
  (if (> _relativelocation_x 100.0)
    (set `self.IsRightMove` false)))

(fn `UserConstructionScript`)