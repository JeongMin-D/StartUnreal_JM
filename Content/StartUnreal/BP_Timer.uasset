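; BP_Timer is a stopwatch that prints elapsed minutes and seconds with Korean unit labels.
; On BeginPlay it binds to the pawn's ClickY event dispatcher, apparently to the generated function that toggles IsPlay to start or pause.
; While playing, Tick calls CountDown, which despite its name adds Speed-scaled delta time to a running total.
; It prints only when the formatted string differs from the previous one.
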(event `self.ReceiveTick`
  (params (DeltaSeconds :type "Float (single-precision)"))
  (if (`self.isPlay`)
    (`self.CountDown` DeltaSeconds)))

(event `self.ReceiveBeginPlay`
  (add `/Game/StartUnreal/BP_Pawn.EventDispatcher_ClickY` (`self.Pawn`) (`|CreateDelegate` :!event `BP_Timer_AutoGenFunc`)))

(fn `BP_Timer_AutoGenFunc`
  (set `self.isPlay` (not (`self.isPlay`))))

(fn `CountDown`
  (params (DeltaSeconds :type "Float (double-precision)"))
  (bind _output_get (set `self.TotalDeltaSeconds` (+ (* DeltaSeconds (`self.Speed`)) (`self.TotalDeltaSeconds`))))
  (bind _returnvalue (`KismetStringLibrary.Concat_StrStr` (`KismetStringLibrary.Conv_IntToString` (`KismetMathLibrary.FFloor` (/ _output_get 60.0))) "분" (`KismetStringLibrary.Conv_IntToString` (`KismetMathLibrary.FFloor` (mod _output_get 60.0))) "초"))
  (if (not (`KismetStringLibrary.EqualEqual_StrStr` _returnvalue (`self.BeforeStr`)))
    (`KismetSystemLibrary.PrintString` _returnvalue)
    (set `self.BeforeStr` _returnvalue)))

(fn `UserConstructionScript`)